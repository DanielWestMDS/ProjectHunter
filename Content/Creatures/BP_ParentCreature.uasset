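; Base creature Blueprint for capturing animals with runes and selling them for currency.
; A rune hitting the hitbox spawns a cage effect and flags BeingCaptured on the AI blackboard.
; Tick shrinks the cage's height as a break timer; expiry frees the creature and resets the player's capture state.
; DestroyCreature credits the sell price to the game instance, increments the player's collected count, plays the capture sound and removes the actor.
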(event OnComponentBeginOverlap(Hitbox)
  (params (OverlappedComponent :type Primitive%20Component%20Object%20Reference) (OtherActor :type Actor%20Object%20Reference) (OtherComp :type Primitive%20Component%20Object%20Reference) (OtherBodyIndex :type Integer) (bFromSweep :type Boolean) (SweepResult :type Hit%20Result%20Structure%20%28by%20ref%29))
  ;[0 0.4328 1] On  rune hit
  (if (not (Variables|Default|GetIsCaptured))
    (bind _asbp_rune (Utilities|Casting|CastToBP_Rune OtherActor))
    (CallFunction|SpawnCage)
    (AI|Components|Blackboard|SetValueasBool (AI|GetBlackboard 0) (Utilities|Name|MakeLiteralName "BeingCaptured") true)
    (Variables|Default|SetIsCaptured true)
    (Actor|DestroyActor _asbp_rune)))

(event Custom|SpawnCage
  (bind _returnvalue (Transformation|GetActorLocation))
  (bind _creaturesize (Variables|Default|GetCreatureSize))
  (bind _returnvalue_2 (Niagara|SpawnSystematLocation "/Game/ProjectHunter/VFX/VFX_Capture.VFX_Capture" (Math|Vector|MakeVector (.x _returnvalue) (.y _returnvalue) (- (.z _returnvalue) 5e+01)) "0, 0, 0" (Math|Vector|MakeVector _creaturesize _creaturesize 1.0)))
  (Variables|Default|SetCageVFX _returnvalue_2)
  (Variables|Default|SetIsCaptured true))

(event Custom|DestroyCreature
  (bind _idnum (Variables|Default|GetIDnum))
  (bind _sellprice (Variables|Default|GetSellPrice))
  ;[1 1 1] Gain money from creature
  (bind _asbp_game_instance (Utilities|Casting|CastToBP_GameInstance (Game|GetGameInstance)))
  (Variables|/Game/gamemode/BP_GameInstance.BP_GameInstance_C|SetCurrency _asbp_game_instance (+ (Variables|/Game/gamemode/BP_GameInstance.BP_GameInstance_C|GetCurrency _asbp_game_instance) _sellprice))
  (Variables|/Game/gamemode/BP_GameInstance.BP_GameInstance_C|SetRound%20Earnings _asbp_game_instance (+ (Variables|/Game/gamemode/BP_GameInstance.BP_GameInstance_C|GetRound%20Earnings _asbp_game_instance) _sellprice))
  (bind _asbp_first_person_character (Utilities|Casting|CastToBP_FirstPersonCharacter (Game|GetPlayerCharacter 0)))
  ;[1 1 1] Add to collected animals
  (bind _result (Math|Integer|IncrementInt (Utilities|Array|Get(acopy) (Variables|/Game/FirstPerson/Blueprints/BP_FirstPersonCharacter.BP_FirstPersonCharacter_C|GetCollectedAnimals _asbp_first_person_character) _idnum))
    (:%20%20
      (Utilities|Array|SetArrayElem (Variables|/Game/FirstPerson/Blueprints/BP_FirstPersonCharacter.BP_FirstPersonCharacter_C|GetCollectedAnimals _asbp_first_person_character) _idnum _result)
      ;[1 1 1] Claim sound
      (Utilities|IsValid (Variables|/Game/FirstPerson/Blueprints/BP_FirstPersonCharacter.BP_FirstPersonCharacter_C|GetCaptureSound _asbp_first_person_character)
        (:Is%20Valid
          (Components|Activation|SetActive (Variables|/Game/FirstPerson/Blueprints/BP_FirstPersonCharacter.BP_FirstPersonCharacter_C|GetCaptureSound _asbp_first_person_character) false true))
        (:Is%20Not%20Valid
          _))
      (Audio|PlaySoundatLocation "/Game/Audio/SFX/Capture_End.Capture_End" (Transformation|GetWorldLocation (Variables|Character|GetMesh)) "0, 0, 0" 1.0 1.0 0.0 0 0 0 0)
      ;[1 1 1] Despawn Cage
      (Utilities|IsValid (Variables|Default|GetCageVFX)
        (:Is%20Valid
          (Components|DestroyComponent (Variables|Default|GetCageVFX)))
        (:Is%20Not%20Valid
          _))
      ;[1 1 1] Destroy
      (Actor|DestroyActor))))

(event EventBeginPlay
  (Variables|Default|SetBreakTimer (Variables|Default|GetBreakTime)))

(event EventTick
  (params (DeltaSeconds :type Float%20%28single-precision%29))
  (bind _creaturesize (Variables|Default|GetCreatureSize))
  (if (Variables|Default|GetIsCaptured)
    (Utilities|IsValid (Variables|Default|GetCageVFX)
      (:Is%20Valid
        ;[1 1 1] Make cage get smaller over time
        (bind _output_get (Variables|Default|SetBreakTimer (- (Variables|Default|GetBreakTimer) (Utilities|Time|GetWorldDeltaSeconds))))
        (Transformation|SetWorldScale3D (Variables|Default|GetCageVFX) (Math|Vector|MakeVector _creaturesize _creaturesize (/ _output_get (Variables|Default|GetBreakTime))))
        (if (<= (Variables|Default|GetBreakTimer) 0.0)
          (AI|Components|Blackboard|SetValueasBool (AI|GetBlackboard 0) (Utilities|Name|MakeLiteralName "BeingCaptured") false)
          (Variables|Default|SetBreakTimer (Variables|Default|GetBreakTime))
          (Components|DestroyComponent (Variables|Default|GetCageVFX))
          (Variables|Default|SetIsCaptured false)
          (bind _asbp_first_person_character (Utilities|Casting|CastToBP_FirstPersonCharacter (Game|GetPlayerCharacter 0)))
          (Variables|/Game/FirstPerson/Blueprints/BP_FirstPersonCharacter.BP_FirstPersonCharacter_C|SetReloadTime _asbp_first_person_character 3.0)
          (Variables|/Game/FirstPerson/Blueprints/BP_FirstPersonCharacter.BP_FirstPersonCharacter_C|SetnoShootAni _asbp_first_person_character true)
          (Utilities|IsValid (Variables|/Game/FirstPerson/Blueprints/BP_FirstPersonCharacter.BP_FirstPersonCharacter_C|GetCaptureSound _asbp_first_person_character)
            (:Is%20Valid
              (Audio|Components|Audio|Stop (Variables|/Game/FirstPerson/Blueprints/BP_FirstPersonCharacter.BP_FirstPersonCharacter_C|GetCaptureSound _asbp_first_person_character)))))))))

(fn ConstructionScript)