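; BP_Reroll is a merchant actor that presents an option to reroll the items for a price.
; UpdatePrice rebuilds the Description text from RerollPrice and plays the reroll sound in 2D.
; BeginPlay calls UpdatePrice after the parent's BeginPlay, so the sound also plays on spawn.
; The reroll and purchase logic is not in this graph, and the overlap and Tick events are disabled.
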(event Custom|UpdatePrice
  (bind _output_get (Variables|Default|SetDescription "Reroll the items. 
 
Price: "))
  (Variables|Default|SetDescription (Utilities|String|Append _output_get (Utilities|String|ToString(Integer) (Variables|Default|GetRerollPrice))))
  (Audio|PlaySound2D "/Game/Audio/SFX/RerollSFX.RerollSFX" 1.0 1.0 0.0 0 0))

(event EventBeginPlay
  (|CallParentFunction)
  (CallFunction|UpdatePrice))

(event Collision|EventActorBeginOverlap
  (params (OtherActor :type Actor%20Object%20Reference))
  (|CallParentFunction OtherActor) ; This node is disabled and will not be called.\nDrag off pins to build functionality.
)

(event EventTick
  (params (DeltaSeconds :type Float%20%28single-precision%29))
  (|CallParentFunction DeltaSeconds) ; This node is disabled and will not be called.\nDrag off pins to build functionality.
)

(fn ConstructionScript
  (|CallParentFunction))